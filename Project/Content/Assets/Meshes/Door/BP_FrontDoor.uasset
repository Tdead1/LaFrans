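; Front door actor that shows a neighbour, train or police figure moving across its plane when the matching game mode event fires.
; BeginPlay binds the three BP_GameMode events and applies a dynamic MM_FrontDoor material to the plane.
; Each handler waits that event's game mode delay, swaps the texture, then drives PanningSpeed forward, back and to zero on short timed delays.
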(event `self.ReceiveBeginPlay`
  (bind _output_get (set `self.Gamemode` (cast `/Game/Player/BP_GameMode` (`GameplayStatics.GetGameMode`) :!pure true)))
  (add `/Game/Player/BP_GameMode.Neighbour` _output_get (delegate `NeighbourSign`))
  (add `/Game/Player/BP_GameMode.Train` _output_get (delegate `TrainSign`))
  (add `/Game/Player/BP_GameMode.Police` _output_get (delegate `PoliceSign`))
  (bind _returnvalue (`KismetMaterialLibrary.CreateDynamicMaterialInstance` "/Game/Assets/Meshes/Door/MM_FrontDoor.MM_FrontDoor"))
  (bind _output_get_2 (set `self.DoorMat` _returnvalue))
  (`PrimitiveComponent.SetMaterial` (`self.Plane`) 0 _output_get_2))

(event `NeighbourSign`
  (bind _doormat (`self.DoorMat`))
  (`KismetSystemLibrary.Delay` (`/Game/Player/BP_GameMode.NeighbourDelay` (cast `/Game/Player/BP_GameMode` (`GameplayStatics.GetGameMode`) :!pure true)))
  (`MaterialInstanceDynamic.SetTextureParameterValue` (`self.DoorMat`) "Texture" (`self.NeighbourMan`))
  (`MaterialInstanceDynamic.SetScalarParameterValue` _doormat "PanningSpeed" 3.0)
  (`KismetSystemLibrary.Delay` 0.5)
  (`MaterialInstanceDynamic.SetScalarParameterValue` _doormat "PanningSpeed" -3.0)
  (`KismetSystemLibrary.Delay` 0.484)
  (`MaterialInstanceDynamic.SetScalarParameterValue` _doormat "PanningSpeed" 0.0))

(event `TrainSign`
  (bind _doormat (`self.DoorMat`))
  (`KismetSystemLibrary.Delay` (`/Game/Player/BP_GameMode.TrainDelay` (cast `/Game/Player/BP_GameMode` (`GameplayStatics.GetGameMode`) :!pure true)))
  (`MaterialInstanceDynamic.SetTextureParameterValue` (`self.DoorMat`) "Texture" (`self.TrainMan`))
  (`MaterialInstanceDynamic.SetScalarParameterValue` _doormat "PanningSpeed" 3.0)
  (`KismetSystemLibrary.Delay` 0.5)
  (`MaterialInstanceDynamic.SetScalarParameterValue` _doormat "PanningSpeed" -3.0)
  (`KismetSystemLibrary.Delay` 0.484)
  (`MaterialInstanceDynamic.SetScalarParameterValue` _doormat "PanningSpeed" 0.0))

(event `PoliceSign`
  (bind _doormat (`self.DoorMat`))
  (`KismetSystemLibrary.Delay` (`/Game/Player/BP_GameMode.PoliceDelay` (cast `/Game/Player/BP_GameMode` (`GameplayStatics.GetGameMode`) :!pure true)))
  (`MaterialInstanceDynamic.SetTextureParameterValue` (`self.DoorMat`) "Texture" (`self.PoliceMan`))
  (`MaterialInstanceDynamic.SetScalarParameterValue` _doormat "PanningSpeed" 3.0)
  (`KismetSystemLibrary.Delay` 0.5)
  (`MaterialInstanceDynamic.SetScalarParameterValue` _doormat "PanningSpeed" -3.0)
  (`KismetSystemLibrary.Delay` 0.484)
  (`MaterialInstanceDynamic.SetScalarParameterValue` _doormat "PanningSpeed" 0.0))

(fn `UserConstructionScript`)