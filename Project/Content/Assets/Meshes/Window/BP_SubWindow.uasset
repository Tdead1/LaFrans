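; BP_SubWindow is a window actor that reacts when its parent window deactivates, then relays that deactivation onward.
; On BeginPlay it binds to its parent, either a BP_Window or another BP_SubWindow, allowing chains, and creates a dynamic window material.
; The event waits TriggerDelay, pans the material for the rest of a one-second span, stops it and calls its own deactivated event.
; The construction script draws a debug line to the parent.
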(event `self.ReceiveBeginPlay`
  (bind _parentwindow (`self.ParentWindow`))
  (bind _asbp_window (cast `/Game/Assets/Meshes/Window/BP_Window` _parentwindow)
    (:`then`
      (add `/Game/Assets/Meshes/Window/BP_Window.WindowDeactivated` _asbp_window (delegate `SubWindowEvent`)))
    (:`CastFailed`
      (bind _asbp_sub_window (cast `/Game/Assets/Meshes/Window/BP_SubWindow` _parentwindow))
      (add `self.SubWindowDeactivated` _asbp_sub_window (delegate `SubWindowEvent`))))
  (bind _returnvalue (`PrimitiveComponent.CreateDynamicMaterialInstance` (`self.Window`) 0 "/Game/Assets/Meshes/Window/MM_Window.MM_Window" "None"))
  (bind _output_get (set `self.MaterialInstance` _returnvalue))
  (`PrimitiveComponent.SetMaterial` (`self.Window`) 0 _output_get))

(event `SubWindowEvent`
  (`KismetSystemLibrary.Delay` (`self.TriggerDelay`))
  (`MaterialInstanceDynamic.SetScalarParameterValue` (`self.MaterialInstance`) "PanningSpeed" 3.0)
  (`KismetSystemLibrary.Delay` (- 1.0 (`self.TriggerDelay`)))
  (`MaterialInstanceDynamic.SetScalarParameterValue` (`self.MaterialInstance`) "PanningSpeed" 0.0)
  (`self.SubWindowDeactivated`))

(fn `UserConstructionScript`
  (`KismetSystemLibrary.DrawDebugLine` (`self.K2_GetActorLocation`) (`self.K2_GetActorLocation` (`self.ParentWindow`)) (struct :`R` 1.0 :`A` 1.0)))