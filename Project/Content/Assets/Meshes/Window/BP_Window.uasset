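; BP_Window is a window actor that animates its material when a game mode event for its window type fires.
; On BeginPlay it creates a dynamic instance of MM_Window and binds WindowEvent to the Neighbour, Police or Train event on BP_GameMode according to WindowType.
; WindowEvent briefly sets the material's PanningSpeed parameter, resets it to zero after a delay, then calls CallWindowDeactivated.
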(event `self.ReceiveBeginPlay`
  (bind _asbp_game_mode (cast `/Game/Player/BP_GameMode` (`GameplayStatics.GetGameMode`) :!pure true))
  (bind _returnvalue (`PrimitiveComponent.CreateDynamicMaterialInstance` (`self.Window`) 0 "/Game/Assets/Meshes/Window/MM_Window.MM_Window" "None"))
  (bind _output_get (set `self.MaterialInstance` _returnvalue))
  (`PrimitiveComponent.SetMaterial` (`self.Window`) 0 _output_get)
  (switch `/Game/Assets/Meshes/Window/ENUM_WindowType` (`self.WindowType`)
    (:`NewEnumerator0`
      (add `/Game/Player/BP_GameMode.Neighbour` _asbp_game_mode (delegate `WindowEvent`)))
    (:`NewEnumerator1`
      (add `/Game/Player/BP_GameMode.Police` _asbp_game_mode (delegate `WindowEvent`)))
    (:`NewEnumerator2`
      (add `/Game/Player/BP_GameMode.Train` _asbp_game_mode (delegate `WindowEvent`)))))

(event `WindowEvent`
  (`MaterialInstanceDynamic.SetScalarParameterValue` (`self.MaterialInstance`) "PanningSpeed" 3.0)
  (`KismetSystemLibrary.Delay` 1.0)
  (`MaterialInstanceDynamic.SetScalarParameterValue` (`self.MaterialInstance`) "PanningSpeed" 0.0)
  (`self.WindowDeactivated`))

(event `self.ReceiveTick`
  (params (DeltaSeconds :type "Float (single-precision)")))

(fn `UserConstructionScript`)