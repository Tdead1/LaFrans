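; Timed bomb actor that explodes after a delay, damaging and knocking back nearby players, then destroys itself.
; On detonation it spawns particles and sound, then subtracts fixed HP from each BP_Player overlapping ExplosionRadius.
; Knockback launches players away from the sphere, adding velocity scaled by clamped inverse distance and Strength.
; PlayHitSound plays a pitch-randomized reaction per family character type, with Dad picking randomly between two sounds.
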(event `self.ReceiveBeginPlay`
  (bind (_returnvalue_location _returnvalue_rotation) (`KismetMathLibrary.BreakTransform` (`SceneComponent.K2_GetComponentToWorld` (`self.Sphere`))))
  (`KismetSystemLibrary.Delay` (`self.Timer`))
  (`GameplayStatics.SpawnEmitterAtLocation` (`self.Particle effect`) _returnvalue_location _returnvalue_rotation (1.0 1.0 1.0) false)
  (`GameplayStatics.PlaySoundAtLocation` "/Game/Audio/SND_Explosion.SND_Explosion" _returnvalue_location (struct) 1.0 (`KismetMathLibrary.RandomFloatInRange` 0.7 1.3) 0.0 null null null)
  (for _array_element (`PrimitiveComponent.GetOverlappingActors` (`self.ExplosionRadius`) "/Script/Engine.Character")
    (bind _asbp_player (cast `/Game/Player/BP_Player` _array_element :!pure true))
    (set `/Game/Player/BP_Player.HP` (- (`/Game/Player/BP_Player.HP` _asbp_player) 40.0) _asbp_player)
    (bind _returnvalue (`self.K2_GetActorLocation` _array_element))
    (bind _returnvalue_2 (- _returnvalue (`SceneComponent.K2_GetComponentLocation` (`self.Sphere`))))
    (`Character.LaunchCharacter` _asbp_player (* (`KismetMathLibrary.Normal` _returnvalue_2) (* (`KismetMathLibrary.FClamp` (/ 100.0 (`KismetMathLibrary.VSize` _returnvalue_2)) 1.0 100.0) (`self.Strength`))) false false)
    (`self.PlayHitSound` _asbp_player _returnvalue))
  (`self.K2_DestroyActor`))

(fn `UserConstructionScript`)