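; Game mode for a local multiplayer last-one-standing match between family characters (Dad, Mother, Daughter, Toddler), requiring a BP_FrontDoor in the level.
; BeginPlay creates local players from the PlayerStart count, assigns meshes and anim classes, then enables input after an intro.
; Tick fires random police, neighbour or train events on an interval.
; A gated Tick check counts dead players, shows the win widget, then flags controllers as done.
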(event `self.ReceiveBeginPlay`
  (bind _deadplayers (`self.DeadPlayers`))
  (bind _players (`/Game/Player/BP_GameMode.Players` (cast `/Game/Player/BP_GameMode` (`GameplayStatics.GetGameMode`) :!pure true)))
  (bind _returnvalue (- (`KismetArrayLibrary.Array_Length` _players) 1))
  (bind _outactors (`GameplayStatics.GetAllActorsOfClass` "/Game/Assets/Meshes/Door/BP_FrontDoor.BP_FrontDoor_C"))
  (bind _output (`|GetArrayItem` _outactors))
  (`/Engine/EditorBlueprintResources/StandardMacros.IsValid` _output
    (:`Is Valid`
      (set `self.FrontDoor` _output)
      (`GameplayStatics.PlaySound2D` "/Game/Audio/SND_CityAmbience.SND_CityAmbience" 1.0 1.0 0.0 null null)
      (`KismetArrayLibrary.Array_Add` (`self.Controllers`) (`GameplayStatics.GetPlayerController` 0))
      (bind _outactors_2 (`GameplayStatics.GetAllActorsOfClass` "/Script/Engine.PlayerStart"))
      (for _ (range (+ (- (`KismetArrayLibrary.Array_Length` _outactors_2) 2) 1))
        (bind _returnvalue_2 (`GameplayStatics.CreatePlayer` -1))
        (`WidgetBlueprintLibrary.SetInputMode_UIOnlyEx` _returnvalue_2 null "LockAlways")
        (`KismetArrayLibrary.Array_Add` (`self.Controllers`) _returnvalue_2))
      (bind _returnvalue_3 (`|CreateWidget` "/Game/UI/WG_IntroText.WG_IntroText_C"))
      (`UserWidget.AddToViewport` _returnvalue_3 0)
      (bind _outactors_3 (`GameplayStatics.GetAllActorsOfClass` "/Game/Player/BP_Player.BP_Player_C"))
      (for (_array_element _array_index) _outactors_3
        (bind _asbp_player (cast `/Game/Player/BP_Player` _array_element :!pure true))
        (`KismetArrayLibrary.Array_Add` (`self.Players`) _asbp_player)
        (`SceneComponent.K2_SetWorldLocation` (`/Game/Player/BP_Player.Camera` _asbp_player) (-912.0 0.0 715.213013) false false)
        (switch `int` _array_index
          (:`0`
            (bind _mesh (`Character.Mesh` _asbp_player))
            (`SkinnedMeshComponent.SetSkinnedAssetAndUpdate` _mesh "/Game/Assets/Meshes/Characters/SK_Dad.SK_Dad" true)
            (set `/Game/Player/BP_Player.CharacterType` "NewEnumerator0" _asbp_player)
            (`SkeletalMeshComponent.K2_SetAnimInstanceClass` _mesh "/Game/Assets/Meshes/Characters/ABP_Dad.ABP_Dad_C"))
          (:`1`
            (`SkinnedMeshComponent.SetSkinnedAssetAndUpdate` _mesh "/Game/Assets/Meshes/Characters/SK_Mother.SK_Mother" true)
            (set `/Game/Player/BP_Player.CharacterType` "NewEnumerator1" _asbp_player)
            (`SkeletalMeshComponent.K2_SetAnimInstanceClass` _mesh "/Game/Assets/Meshes/Characters/ABP_Mother.ABP_Mother_C"))
          (:`2`
            (`SkinnedMeshComponent.SetSkinnedAssetAndUpdate` _mesh "/Game/Assets/Meshes/Characters/SK_Daughter_new.SK_Daughter_new" true)
            (set `/Game/Player/BP_Player.CharacterType` "NewEnumerator2" _asbp_player)
            (`SkeletalMeshComponent.K2_SetAnimInstanceClass` _mesh "/Game/Assets/Meshes/Characters/ABP_Daughter.ABP_Daughter_C"))
          (:`3`
            (`SkinnedMeshComponent.SetSkinnedAssetAndUpdate` _mesh "/Game/Assets/Meshes/Characters/SK_Toddler.SK_Toddler" true)
            (set `/Game/Player/BP_Player.CharacterType` "NewEnumerator3" _asbp_player)
            (`SceneComponent.SetWorldScale3D` _mesh (20.0 20.0 20.0))
            (`SkeletalMeshComponent.K2_SetAnimInstanceClass` _mesh "/Game/Assets/Meshes/Characters/ABP_Toddler.ABP_Toddler_C")))
        (set `/Game/Player/BP_Player.FrontDoor` (`self.FrontDoor`) _asbp_player))
      (`KismetSystemLibrary.Delay` 3.0)
      (for _array_element_2 (`self.Controllers`)
        (`WidgetBlueprintLibrary.SetInputMode_GameAndUIEx` _array_element_2 null)
        (`Widget.SetVisibility` _returnvalue_3 "Collapsed")
        (bind _returnvalue_4 (`|CreateWidget` "/Game/UI/WG_InGame.WG_InGame_C"))
        (`UserWidget.AddToViewport` _returnvalue_4 0))
      (`GameplayStatics.PlaySound2D` "/Game/Audio/SND_Soundtrack.SND_Soundtrack" 1.0 1.0 0.0 null null)
      (goto _label_2 :!via `Open`))
    (:`Is Not Valid`
      (`KismetSystemLibrary.PrintString` "NO FRONT DOOR DETECTED, GAME WILL NOT WORK."))))

(event `self.ReceiveTick`
  (params (DeltaSeconds :type "Float (single-precision)"))
  (bind _deadplayers (`self.DeadPlayers`))
  (bind _players (`/Game/Player/BP_GameMode.Players` (cast `/Game/Player/BP_GameMode` (`GameplayStatics.GetGameMode`) :!pure true)))
  (bind _returnvalue (- (`KismetArrayLibrary.Array_Length` _players) 1))
  (`|ExecutionSequence`
    (:`then_0`
      (`/Engine/EditorBlueprintResources/StandardMacros.DoOnce` false :!label _label
        (:`Completed`
          (`KismetSystemLibrary.Delay` (- (`KismetSystemLibrary.MakeLiteralDouble` (`self.CurrentEventInterval`)) 0.016))
          (switch `int` (`KismetMathLibrary.RandomInteger` 3)
            (:`0`
              (`self.Police`)
              (goto _label :!via `Reset`))
            (:`1`
              (`self.Neighbour`)
              (goto _label :!via `Reset`))
            (:`2`
              (`self.Train`)
              (goto _label :!via `Reset`))))))
    (:`then_1`
      (`/Engine/EditorBlueprintResources/StandardMacros.Gate` true :!label _label_2
        (:`Exit`
          (if (`self.Won`)
            (`/Engine/EditorBlueprintResources/StandardMacros.DoOnce` false
              (:`Completed`
                (`KismetSystemLibrary.Delay` 3.0)
                (`Widget.SetVisibility` (`/Game/UI/WG_PlayerWins.KeyToContinue` (`self.WinWidget`)) "Visible")
                (for _array_element (`self.Controllers`)
                  (bind _asbp_player_controller (cast `/Game/Player/BP_PlayerController` _array_element))
                  (set `/Game/Player/BP_PlayerController.GameDone` true _asbp_player_controller))))
            (else
              (for _array_element_2 _players
                (if (< (`/Game/Player/BP_Player.HP` _array_element_2) 0.1)
                  (`/Engine/EditorBlueprintResources/StandardMacros.IncrementInt` (`self.DeadPlayers`))
                  (else
                    (set `self.PlayerAlive` (`/Game/Player/BP_Player.CharacterType` _array_element_2)))))
              (if (== _returnvalue _deadplayers)
                (set `self.Won` true)
                (`/Engine/EditorBlueprintResources/StandardMacros.DoOnce` false :!label _label_3
                  (:`Completed`
                    (bind _returnvalue_2 (`|CreateWidget` "/Game/UI/WG_PlayerWins.WG_PlayerWins_C"))
                    (`UserWidget.AddToViewport` _returnvalue_2 0)
                    (`Widget.SetVisibility` _returnvalue_2 "Visible")
                    (set `self.WinWidget` _returnvalue_2)))
                (elif (> _deadplayers _returnvalue)
                  (set `self.Won` true)
                  (set `self.EveryoneDied` true)
                  (goto _label_3)
                  (else
                    (set `self.DeadPlayers` 0)))))))))))

(fn `UserConstructionScript`)