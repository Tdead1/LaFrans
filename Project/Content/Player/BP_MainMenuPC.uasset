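; BP_MainMenuPC is the main menu's player controller, which shows the mouse cursor and puts the WG_MainMenu widget on screen at BeginPlay.
; It keeps a reference to that widget and relays input to it: any key press sets its AnyKey flag, while Escape and the Throw action call its EscPressed and BPressed handlers.
; The movement axis events and Tick are empty.
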(event `self.ReceiveBeginPlay`
  (set `self.bShowMouseCursor` true)
  (bind _returnvalue (`|CreateWidget` "/Game/UI/WG_MainMenu.WG_MainMenu_C" self))
  (`UserWidget.AddToViewport` _returnvalue 0)
  (set `self.Menu` _returnvalue))

(event `InputAction|Jump` :consume false
  (params (Key :type "Key Structure")))

(event `InputAxis|Right` :consume false
  (params (AxisValue :type "Float (single-precision)")))

(event `InputAxis|Forward` :consume false
  (params (AxisValue :type "Float (single-precision)")))

(event `Key|AnyKey` :consume false
  (params (Key :type "Key Structure"))
  (:`Pressed`
    (set `/Game/UI/WG_MainMenu.AnyKey` true (`self.Menu`))))

(event `Key|Escape` :consume false
  (params (Key :type "Key Structure"))
  (:`Pressed`
    (`/Game/UI/WG_MainMenu.EscPressed` (`self.Menu`))))

(event `InputAction|Throw` :consume false
  (params (Key :type "Key Structure"))
  (:`Pressed`
    (`/Game/UI/WG_MainMenu.BPressed` (`self.Menu`))))

(fn `UserConstructionScript`)