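; Player character that handles world-axis movement, jumping and bomb throwing.
; Throw spawns a BP_Bomb launched along the Direction component plus the character's velocity, with a DoOnce and delay acting as cooldown.
; Tick yaws the mesh toward the velocity while moving; mouse look is disconnected.
; Dialogue participant functions are default-returning stubs, and GetCurrentPlayer, used by input handlers, contains only an unwired player-pawn cast.
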(event `InputAxis|Forward`
  (params (AxisValue :type "Float (single-precision)"))
  ;[1 1 1] Input handling
  (`self.AddMovementInput` (`self.GetCurrentPlayer`) (`KismetMathLibrary.MakeVector` AxisValue) 1.0 false))

(event `InputAxis|Right`
  (params (AxisValue :type "Float (single-precision)"))
  ;[1 1 1] Input handling
  (`self.AddMovementInput` (`self.GetCurrentPlayer`) (`KismetMathLibrary.MakeVector` 0.0 AxisValue) 1.0 false))

(event `InputAction|Jump`
  (params (Key :type "Key Structure"))
  ;[1 1 1] Input handling
  (:`Pressed`
    (`self.Jump` (`self.GetCurrentPlayer`))))

(event `InputAxis|MouseX`
  (params (AxisValue :type "Float (single-precision)"))
  ;[1 1 1] Input handling
)

(event `InputAxis|MouseY`
  (params (AxisValue :type "Float (single-precision)"))
  ;[1 1 1] Input handling
)

(event `InputAction|Throw`
  (params (Key :type "Key Structure"))
  (bind _returnvalue (`self.GetCurrentPlayer`))
  ;[1 1 1] Input handling
  (:`Pressed`
    (`/Engine/EditorBlueprintResources/StandardMacros.DoOnce` false :!label _label
      (:`Completed`
        (bind _returnvalue_2 (`|SpawnActorFromClass` "/Game/Player/BP_Bomb.BP_Bomb_C" (`self.GetTransform` _returnvalue) "Undefined" "OverrideRootScale" null null))
        (`PrimitiveComponent.SetAllPhysicsLinearVelocity` (`/Game/Player/BP_Bomb.Sphere` _returnvalue_2) (+ (* (`KismetMathLibrary.GetForwardVector` (`SceneComponent.K2_GetComponentRotation` (`/Game/Player/BP_Player.Direction` _returnvalue))) 800.0) (`MovementComponent.Velocity` (`self.CharacterMovement`))) true)
        (`KismetSystemLibrary.Delay` (`self.BombThrowDelay`))
        (goto _label :!via `Reset`)))))

(event `self.ReceiveTick`
  (params (DeltaSeconds :type "Float (single-precision)"))
  (bind _returnvalue (`self.K2_GetActorLocation`))
  (bind _velocity (`MovementComponent.Velocity` (`self.CharacterMovement`)))
  (bind (_returnvalue_roll _returnvalue_pitch _returnvalue_yaw) (`KismetMathLibrary.BreakRotator` (`KismetMathLibrary.FindLookAtRotation` _returnvalue (+ _velocity _returnvalue))))
  (if (not (< (`KismetMathLibrary.VSizeSquared` _velocity) 100.0))
    (`SceneComponent.K2_SetWorldRotation` (`self.Mesh`) (`KismetMathLibrary.MakeRotator` 0.0 0.0 _returnvalue_yaw) false false)))

(fn `CheckCondition`
  (params (ConditionName :type "Name (by ref)"))
  (returns (ReturnValue :type Boolean))
  (return false))

(fn `GetBoolValue`
  (params (ValueName :type "Name (by ref)"))
  (returns (ReturnValue :type Boolean))
  (return false))

(fn `GetFloatValue`
  (params (ValueName :type "Name (by ref)"))
  (returns (ReturnValue :type "Float (double-precision)"))
  (return 0.0))

(fn `GetIntValue`
  (params (ValueName :type "Name (by ref)"))
  (returns (ReturnValue :type Integer))
  (return 0))

(fn `GetNameValue`
  (params (ValueName :type "Name (by ref)"))
  (returns (ReturnValue :type Name))
  (return "None"))

(fn `GetParticipantDisplayName`
  (params (ActiveSpeaker :type Name))
  (returns (ReturnValue :type Text))
  (return ""))

(fn `GetParticipantGender`
  (returns (ReturnValue :type "ETextGender Enum"))
  (return "Masculine"))

(fn `GetParticipantIcon`
  (params (ActiveSpeaker :type Name) (ActiveSpeakerState :type Name))
  (returns (ReturnValue :type "Texture2D Object Reference"))
  (return null))

(fn `GetParticipantName`
  (returns (ReturnValue :type Name))
  (return "None"))

(fn `ModifyBoolValue`
  (params (ValueName :type "Name (by ref)") (bNewValue :type Boolean))
  (returns (ReturnValue :type Boolean))
  (return false))

(fn `ModifyFloatValue`
  (params (ValueName :type "Name (by ref)") (bDelta :type Boolean) (Value :type "Float (double-precision)"))
  (returns (ReturnValue :type Boolean))
  (return false))

(fn `ModifyIntValue`
  (params (ValueName :type "Name (by ref)") (bDelta :type Boolean) (Value :type Integer))
  (returns (ReturnValue :type Boolean))
  (return false))

(fn `ModifyNameValue`
  (params (ValueName :type "Name (by ref)") (NameValue :type "Name (by ref)"))
  (returns (ReturnValue :type Boolean))
  (return false))

(fn `OnDialogueEvent`
  (params (EventName :type "Name (by ref)"))
  (returns (ReturnValue :type Boolean))
  (return false))

(fn `UserConstructionScript`)